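; BP_PutzleItem is a collectible puzzle item that floats in place and reports its pickup to the puzzle gate.
; Two chained timelines, FloatingAnim forward and DownAnim in reverse, loop to animate the Item component's relative location.
; When a BP_Caption actor overlaps the trigger, it finds BP_PuzzieGate by class, calls CollectItem, plays a camera shutter sound and destroys itself.
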(event `self.ReceiveBeginPlay`
  (bind _item (`self.Item`))
  (bind (_direction _z_axie_anim) (`Timeline|FloatingAnim` :!label _label)
    (:`Update`
      (`SceneComponent.K2_SetRelativeLocation` _item _z_axie_anim false false))
    (:`Finished`
      (bind (_direction_2 _z_axie_anim_2) (`Timeline|downAnim` :!via `ReverseFromEnd`)
        (:`Update`
          (`SceneComponent.K2_SetRelativeLocation` _item _z_axie_anim_2 false false))
        (:`Finished`
          (goto _label :!via `PlayFromStart`))))))

(event `self.Trigget.OnComponentBeginOverlap`
  (params (OverlappedComponent :type "PrimitiveComponent Object Reference") (OtherActor :type "Actor Object Reference") (OtherComp :type "PrimitiveComponent Object Reference") (OtherBodyIndex :type Integer) (bFromSweep :type Boolean) (SweepResult :type "HitResult Structure (by ref)"))
  (cast `/Game/Blueprint/Character/caption/BP_Caption` OtherActor)
  (bind _returnvalue (`GameplayStatics.GetActorOfClass` "/Game/Blueprint/Event/BP_PuzzieGate.BP_PuzzieGate_C"))
  (`/Game/Blueprint/Event/BP_PuzzieGate.Collect Item` _returnvalue)
  (`GameplayStatics.PlaySound2D` "/Engine/VREditor/Sounds/UI/Camera_Shutter.Camera_Shutter" 1.0 1.0 0.0 null null)
  (`self.K2_DestroyActor`))

(fn `UserConstructionScript`)