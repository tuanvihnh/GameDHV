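; BP_chest is a Paper2D chest pickup that rewards the player character with random experience.
; BeginPlay caches the player as BP_Caption; GetPicked toggles IsClosed and, when it becomes true, swaps the flipbook, adds the experience and triggers destruction after a short delay.
; That branch returns item name, ID, experience gained and player level.
; Interact is empty, and ShowNextLine always returns false.
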(event `self.ReceiveBeginPlay`
  (bind _asbp_caption (cast `/Game/Blueprint/Character/caption/BP_Caption` (`GameplayStatics.GetPlayerCharacter` 0)))
  (set `self.character` _asbp_caption))

(event `Delay`
  (`KismetSystemLibrary.Delay` 3.0)
  (`self.K2_DestroyActor`))

(event `/Game/Blueprint/Interfaces/BPI_InterAction.Interact`
  (params (Instigator :type "/Game/Blueprint/Character/BP_ActionChar Object Reference")))

(fn `GetPicked`
  (returns (ItemName :type String) (ItemID :type Integer) (ExpRandom :type "Float (double-precision)") (Level :type "Float (double-precision)"))
  (bind _character (`self.character`))
  (bind _output_get (set `self.isClosed` (not (`self.isClosed`))))
  (if _output_get
    (`PaperFlipbookComponent.SetFlipbook` (`self.RenderComponent`) "/Game/PaperAssets/Item/Chest/mo.mo")
    (bind _output_get_2 (set `self.isClosed` true))
    (if _output_get_2
      (bind _output_get_3 (set `self.RandomExp` (`KismetMathLibrary.RandomFloatInRange` 50.0 100.0)))
      (`/Game/Blueprint/Character/caption/BP_Caption.AddExp` _character _output_get_3)
      (`self.Delay`)
      (return (`self.ItemName`) (`self.ItemID`) (`self.RandomExp`) (`/Game/Blueprint/Character/BP_ActionChar.Level` _character)))))

(fn `ShowNextLine`
  (returns (HasNextLine :type Boolean))
  (return false))

(fn `UserConstructionScript`)