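; BP_SpawnShark is a spawn point that releases queued shark classes just above its static mesh for the wave game mode.
; AddSharkToQueue spawns at once if no BP_Shark overlaps its sphere, while a looping one-second timer drains the queue without that check.
; Each spawn binds an elimination event, with OnSharkEliminated forwarding to the wave game mode.
; Spawned sharks are tracked so ClearAllShark can destroy them.
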(event `self.ReceiveBeginPlay`
  (`KismetSystemLibrary.K2_SetTimerDelegate` (delegate `TrySpawnShark`) 1.0 true))

(event `TrySpawnShark`
  (`self.SpawnShark`))

(event `Clear All Shark`
  (for _array_element (`self.SpawnedShark`)
    (`/Engine/EditorBlueprintResources/StandardMacros.IsValid` _array_element
      (:`Is Valid`
        (`self.K2_DestroyActor` _array_element)))))

(event `OnSharkEliminated`
  (`/Game/Blueprint/GM_Action.OnSharkEliminated` (`/Game/Blueprint/BP_FuntionLibrary.GetWaveGameMode`)))

(fn `AddSharkToQueue`
  (params (SharkClass :type "/Game/Blueprint/Character/Shark/BP_Shark Class Reference (by ref)"))
  (`KismetArrayLibrary.Array_Add` (`self.SharkQueue`) SharkClass)
  (if (not (`KismetArrayLibrary.Array_IsValidIndex` (`PrimitiveComponent.GetOverlappingActors` (`self.SphereCollision`) "/Game/Blueprint/Character/Shark/BP_Shark.BP_Shark_C")))
    (`self.SpawnShark`)))

(fn `SpawnShark`
  (returns (Success :type Boolean))
  (bind (_returnvalue_x _returnvalue_y _returnvalue_z) (`KismetMathLibrary.BreakVector` (`SceneComponent.K2_GetComponentLocation` (`self.StaticMesh`))))
  (if (`KismetArrayLibrary.Array_IsValidIndex` (`self.SharkQueue`))
    (bind _returnvalue (`|SpawnActorFromClass` (`|GetArrayItem` (`self.SharkQueue`)) (`KismetMathLibrary.MakeTransform` (`KismetMathLibrary.MakeVector` _returnvalue_x _returnvalue_y (+ _returnvalue_z 60.0))) "AdjustIfPossibleButAlwaysSpawn" "MultiplyWithRoot" null null))
    (`/Engine/EditorBlueprintResources/StandardMacros.IsValid` _returnvalue
      (:`Is Valid`
        (add `/Game/Blueprint/Character/Shark/BP_Shark.OnElminated` _returnvalue (`|CreateDelegate` :!event `OnSharkEliminated`))
        (`KismetArrayLibrary.Array_Remove` (`self.SharkQueue`))
        (`KismetArrayLibrary.Array_Add` (`self.SpawnedShark`) _returnvalue)
        (return true)))
    (else
      (return false))))

(fn `UserConstructionScript`)