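; BP_chest1 is a flipbook-based treasure chest item that rewards the player with experience and triggers shark spawns when picked.
; GetPicked toggles IsClosed and, when it becomes true, swaps the flipbook, grants random experience to the cached BP_Caption player and calls SpawnShark on every BP_Spawner.
; It then returns the item name, ID, experience and player level, while a custom Delay event destroys the chest three seconds later.
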(event `self.ReceiveBeginPlay`
  (bind _asbp_caption (cast `/Game/Blueprint/Character/caption/BP_Caption` (`GameplayStatics.GetPlayerCharacter` 0)))
  (set `self.character` _asbp_caption))

(event `Delay`
  (`KismetSystemLibrary.Delay` 3.0)
  (`self.K2_DestroyActor`))

(fn `GetPicked`
  (returns (ItemName :type String) (ItemID :type Integer) (ExpRandom :type "Float (double-precision)") (Level :type "Float (double-precision)"))
  (bind _character (`self.character`))
  (bind _output_get (set `self.isClosed` (not (`self.isClosed`))))
  (if _output_get
    (`PaperFlipbookComponent.SetFlipbook` (`self.PaperFlipbook`) "/Game/PaperAssets/Item/Chest/mo.mo")
    (bind _output_get_2 (set `self.isClosed` true))
    (if _output_get_2
      (bind _output_get_3 (set `self.RandomExp` (`KismetMathLibrary.RandomFloatInRange` 50.0 100.0)))
      (`/Game/Blueprint/Character/caption/BP_Caption.AddExp` _character _output_get_3)
      (bind _outactors (`GameplayStatics.GetAllActorsOfClass` "/Game/Blueprint/Event/BP_Spawner.BP_Spawner_C"))
      (for _array_element _outactors
        (`/Game/Blueprint/Event/BP_Spawner.SpawnShark` _array_element))
      (`self.Delay`)
      (return (`self.ItemName`) (`self.ItemID`) (`self.RandomExp`) (`/Game/Blueprint/Character/BP_ActionChar.Level` _character)))))

(fn `ShowNextLine`
  (returns (HasNextLine :type Boolean))
  (return false))

(fn `UserConstructionScript`)