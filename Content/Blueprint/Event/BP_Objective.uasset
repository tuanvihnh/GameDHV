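; BP_Objective is a one-shot trigger box that hands the player a new objective and starts a puzzle sequence.
; When a BP_Caption actor outside a safe zone overlaps it, it sets the objective on the linked character and reveals the objectives text.
; It finds the puzzle gate and three puzzle items by class, closes the gate, unhides the items, calls SlideOn, plays a shutter sound and destroys itself.
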(event `self.Box.OnComponentBeginOverlap`
  (params (OverlappedComponent :type "PrimitiveComponent Object Reference") (OtherActor :type "Actor Object Reference") (OtherComp :type "PrimitiveComponent Object Reference") (OtherBodyIndex :type Integer) (bFromSweep :type Boolean) (SweepResult :type "HitResult Structure (by ref)"))
  (bind _asbp_caption (cast `/Game/Blueprint/Character/caption/BP_Caption` OtherActor))
  (if (not (`/Game/Blueprint/Character/BP_ActionChar.IsInSafeZone?` _asbp_caption))
    (bind _charref (`/Game/Blueprint/Character/caption/BP_Caption.CharRef` _asbp_caption))
    (set `/Game/Blueprint/GM_Action.CurrentObjective` (`self.Objective`) _charref)
    (`Widget.SetVisibility` (`/Game/Widget/WB_Quest.TextBlock_102` (`/Game/Blueprint/GM_Action.Objectives Widget REF` _charref)) "Visible")
    (bind _returnvalue (`GameplayStatics.GetActorOfClass` "/Game/Blueprint/Event/BP_PuzzieGate.BP_PuzzieGate_C"))
    (`/Game/Blueprint/Event/BP_PuzzieGate.Close Door` _returnvalue)
    (bind _returnvalue_2 (`GameplayStatics.GetActorOfClass` "/Game/Blueprint/Event/BP_PutzleItem.BP_PutzleItem_C"))
    (bind _returnvalue_3 (`GameplayStatics.GetActorOfClass` "/Game/Blueprint/Event/BP_PutzleItem2.BP_PutzleItem2_C"))
    (bind _returnvalue_4 (`GameplayStatics.GetActorOfClass` "/Game/Blueprint/Event/BP_PutzleItem3.BP_PutzleItem3_C"))
    (`/Game/Blueprint/Event/BP_PutzleItem.NoHide` _returnvalue_2)
    (`/Game/Blueprint/Event/BP_PutzleItem.NoHide` _returnvalue_3)
    (`/Game/Blueprint/Event/BP_PutzleItem.NoHide` _returnvalue_4)
    (`/Game/Blueprint/GM_Action.Slide On` _charref)
    (`GameplayStatics.PlaySound2D` "/Engine/VREditor/Sounds/UI/Camera_Shutter.Camera_Shutter" 1.0 1.0 0.0 null null)
    (`self.K2_DestroyActor`)))

(fn `UserConstructionScript`)