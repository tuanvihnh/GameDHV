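; Checkpoint actor that sets a BP_Caption's respawn location when it enters the trigger box.
; On overlap it loops over all Respawn_Point actors, breaking if one is the overlapping actor and otherwise writing its own Arrow location to the character's RespawnPoint.
; Activate and Deactivate spawn and destroy a Niagara effect at the ParticleSystem transform, but nothing in this graph calls them.
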(event `self.Box.OnComponentBeginOverlap`
  (params (OverlappedComponent :type "PrimitiveComponent Object Reference") (OtherActor :type "Actor Object Reference") (OtherComp :type "PrimitiveComponent Object Reference") (OtherBodyIndex :type Integer) (bFromSweep :type Boolean) (SweepResult :type "HitResult Structure (by ref)"))
  (bind _outactors (`GameplayStatics.GetAllActorsOfClass` "Respawn_Point_C"))
  (for _array_element _outactors :!label _label
    (if (== _array_element OtherActor)
      (`self.Break`)
      (else
        (bind _asbp_caption (cast `/Game/Blueprint/Character/caption/BP_Caption` OtherActor))
        (set `/Game/Blueprint/Character/caption/BP_Caption.RespawnPoint` (`SceneComponent.K2_GetComponentLocation` (`self.Arrow`)) _asbp_caption)))))

(event `Break`
  (goto _label :!via `Break`))

(event `Activate`
  (bind (_returnvalue_location _returnvalue_rotation _returnvalue_scale) (`KismetMathLibrary.BreakTransform` (`SceneComponent.K2_GetComponentToWorld` (`self.ParticleSystem`))))
  (`/Engine/EditorBlueprintResources/StandardMacros.IsValid` (`self.TeleportSS`)
    (:`Is Not Valid`
      (bind _returnvalue (`NiagaraFunctionLibrary.SpawnSystemAtLocation` "/Game/Basic_VFX/Niagara/NS_Basic_14.NS_Basic_14" _returnvalue_location _returnvalue_rotation _returnvalue_scale))
      (set `self.TeleportSS` _returnvalue))))

(event `Deactivate`
  (bind _teleportss (`self.TeleportSS`))
  (`/Engine/EditorBlueprintResources/StandardMacros.IsValid` _teleportss
    (:`Is Valid`
      (`ActorComponent.K2_DestroyComponent` _teleportss))))

(fn `UserConstructionScript`)