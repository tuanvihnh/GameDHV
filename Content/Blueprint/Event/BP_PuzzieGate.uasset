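; Puzzle gate that opens once the player has collected every required item and leads to the end of the game.
; CollectItem increments the counter on BP_Caption's CharRef; at the maximum it fires OpenDoor once, plus SlideOff and QuestMisstion.
; OpenDoor pitches the door to 90 degrees via timeline, while CloseDoor's lerp holds zero throughout.
; BP_Caption overlapping Trigger plays a sound, fades in WB_EndGame, then loads EndGame after a delay.
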(event `Open Door`
  (bind (_direction _door_rotation) (`Timeline|OpenDoorAnimation`)
    (:`Update`
      (`SceneComponent.K2_SetRelativeRotation` (`self.Door`) (`KismetMathLibrary.MakeRotator` 0.0 (`KismetMathLibrary.Lerp` 0.0 90.0 _door_rotation)) false false))))

(event `Close Door`
  (bind (_direction _door_rotation) (`Timeline|Timeline`)
    (:`Update`
      (`SceneComponent.K2_SetRelativeRotation` (`self.Door`) (`KismetMathLibrary.MakeRotator` 0.0 (`KismetMathLibrary.Lerp` 0.0 0.0 _door_rotation)) false false))))

(event `Collect Item`
  (bind _asbp_caption (cast `/Game/Blueprint/Character/caption/BP_Caption` (`GameplayStatics.GetPlayerCharacter` 0)))
  (bind _charref (`/Game/Blueprint/Character/caption/BP_Caption.CharRef` _asbp_caption))
  (`/Engine/EditorBlueprintResources/StandardMacros.IncrementInt` (`/Game/Blueprint/GM_Action.CurrentItemsCollected` _charref)
    (:`  `
      (if (>= (`/Game/Blueprint/GM_Action.CurrentItemsCollected` _charref) (`/Game/Blueprint/GM_Action.maxItemsCollectable` _charref))
        (`/Engine/EditorBlueprintResources/StandardMacros.DoOnce` false
          (:`Completed`
            (`self.Open Door`)
            (`/Game/Blueprint/GM_Action.Slide Off` _charref)
            (`/Game/Blueprint/GM_Action.QuestMisstion` _charref)))))))

(event `self.Trigger.OnComponentBeginOverlap`
  (params (OverlappedComponent :type "PrimitiveComponent Object Reference") (OtherActor :type "Actor Object Reference") (OtherComp :type "PrimitiveComponent Object Reference") (OtherBodyIndex :type Integer) (bFromSweep :type Boolean) (SweepResult :type "HitResult Structure (by ref)"))
  (cast `/Game/Blueprint/Character/caption/BP_Caption` OtherActor)
  (`GameplayStatics.PlaySound2D` "/Engine/VREditor/Sounds/UI/Dockable_Window_Drop.Dockable_Window_Drop" 1.0 1.0 0.0 null null)
  (bind _returnvalue (`|CreateWidget` "/Game/Widget/WB_EndGame.WB_EndGame_C"))
  (`UserWidget.AddToViewport` _returnvalue 0)
  (`/Game/Widget/WB_EndGame.Fade Anim` _returnvalue)
  (`KismetSystemLibrary.Delay` 1.0)
  (`GameplayStatics.OpenLevel` "EndGame"))

(fn `UserConstructionScript`)