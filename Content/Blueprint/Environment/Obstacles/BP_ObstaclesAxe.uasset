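; Axe obstacle that swings or spins and damages any BP_Caption it touches.
; With RotateFully off, it stops RotatingMovement and a timeline endlessly ping-pongs the Cylinder's yaw through a half-circle arc; otherwise RotatingMovement is left active.
; Two overlap boxes call ReceiveAttack with different damage amounts.
; The Swingtime timeline-length setter is never executed.
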(event `self.ReceiveBeginPlay`
  (if (not (`self.RotateFully`))
    (`self.AxeSwing`)
    (set `RotatingMovementComponent.RotationRate` (struct) (`self.RotatingMovement`))))

(event `AxeSwing`
  (set `self.Direction` "Forward")
  (bind (_direction _newtrack_0) (`Timeline|AxeSwingAnimation` :!label _label)
    (:`Update`
      (`SceneComponent.K2_SetRelativeRotation` (`self.Cylinder`) (`KismetMathLibrary.MakeRotator` 0.0 0.0 (`KismetMathLibrary.Lerp` -90.0 90.0 _newtrack_0)) false false))
    (:`Finished`
      (if (not (`|EnumEquality` _direction "Forward"))
        (`self.AxeSwing`)
        (else
          (`self.ReverseAxeSwing`))))))

(event `ReverseAxeSwing`
  (set `self.Direction` "Backward")
  (goto _label :!via `Reverse`))

(event `self.Box.OnComponentBeginOverlap`
  (params (OverlappedComponent :type "PrimitiveComponent Object Reference") (OtherActor :type "Actor Object Reference") (OtherComp :type "PrimitiveComponent Object Reference") (OtherBodyIndex :type Integer) (bFromSweep :type Boolean) (SweepResult :type "HitResult Structure (by ref)"))
  (bind _asbp_caption (cast `/Game/Blueprint/Character/caption/BP_Caption` OtherActor))
  (`/Game/Blueprint/Character/BP_ActionChar.ReceiveAttack` _asbp_caption 25.0))

(event `self.Box1.OnComponentBeginOverlap`
  (params (OverlappedComponent :type "PrimitiveComponent Object Reference") (OtherActor :type "Actor Object Reference") (OtherComp :type "PrimitiveComponent Object Reference") (OtherBodyIndex :type Integer) (bFromSweep :type Boolean) (SweepResult :type "HitResult Structure (by ref)"))
  (bind _asbp_caption (cast `/Game/Blueprint/Character/caption/BP_Caption` OtherActor))
  (`/Game/Blueprint/Character/BP_ActionChar.ReceiveAttack` _asbp_caption 10.0))

(fn `UserConstructionScript`)