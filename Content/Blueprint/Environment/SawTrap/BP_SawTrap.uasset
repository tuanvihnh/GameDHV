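; BP_SawTrap is an environmental hazard with a moving, spinning saw that hurts BP_Caption actors.
; On BeginPlay it starts two timelines: one slides the saw between two relative positions along local X, the other drives its pitch rotation.
; A Box overlap casts the other actor to BP_Caption and calls its ReceiveAttack with a fixed value.
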(event `self.ReceiveBeginPlay`
  (bind _saw (`self.Saw`))
  (`|ExecutionSequence`
    (:`then_0`
      (bind (_direction _move) (`Timeline|LeftAndRight`)
        (:`Update`
          (`SceneComponent.K2_SetRelativeLocation` _saw (`KismetMathLibrary.VLerp` (0.0 0.0 0.0) (234.0 0.0 0.0) _move) false false))))
    (:`then_1`
      (bind (_direction_2 _rotation) (`Timeline|Rotation`)
        (:`Update`
          (`SceneComponent.K2_SetRelativeRotation` _saw (`KismetMathLibrary.MakeRotator` 0.0 _rotation) false false))))))

(event `self.Box.OnComponentBeginOverlap`
  (params (OverlappedComponent :type "PrimitiveComponent Object Reference") (OtherActor :type "Actor Object Reference") (OtherComp :type "PrimitiveComponent Object Reference") (OtherBodyIndex :type Integer) (bFromSweep :type Boolean) (SweepResult :type "HitResult Structure (by ref)"))
  (bind _asbp_caption (cast `/Game/Blueprint/Character/caption/BP_Caption` OtherActor))
  (`/Game/Blueprint/Character/BP_ActionChar.ReceiveAttack` _asbp_caption 10.0))

(fn `UserConstructionScript`)