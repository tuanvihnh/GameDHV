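; BP_Door is a door that opens once the player has collected the required number of items.
; Its CollectItem event increments the count on the BP_Caption player's CharRef and compares it to the maximum.
; Reaching the maximum fires a one-time trigger that calls OpenDoor, SlideOff and QuestMisstion.
; OpenDoor plays a timeline that swings the door a quarter turn on its relative pitch axis.
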(event `Open Door`
  (bind (_direction _door_rotation) (`Timeline|OpenDoorAnimation`)
    (:`Update`
      (`SceneComponent.K2_SetRelativeRotation` (`self.Door`) (`KismetMathLibrary.MakeRotator` 0.0 (`KismetMathLibrary.Lerp` 0.0 90.0 _door_rotation)) false false))))

(event `Collect Item`
  (bind _asbp_caption (cast `/Game/Blueprint/Character/caption/BP_Caption` (`GameplayStatics.GetPlayerCharacter` 0)))
  (bind _charref (`/Game/Blueprint/Character/caption/BP_Caption.CharRef` _asbp_caption))
  (`/Engine/EditorBlueprintResources/StandardMacros.IncrementInt` (`/Game/Blueprint/GM_Action.CurrentItemsCollected` _charref)
    (:`  `
      (if (>= (`/Game/Blueprint/GM_Action.CurrentItemsCollected` _charref) (`/Game/Blueprint/GM_Action.maxItemsCollectable` _charref))
        (`/Engine/EditorBlueprintResources/StandardMacros.DoOnce` false
          (:`Completed`
            (`self.Open Door`)
            (`/Game/Blueprint/GM_Action.Slide Off` _charref)
            (`/Game/Blueprint/GM_Action.QuestMisstion` _charref)))))))

(fn `UserConstructionScript`)