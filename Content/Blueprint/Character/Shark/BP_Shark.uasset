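; Shark enemy character that targets the player's BP_Caption through its AI controller when they enter its aggro range.
; A world-space health bar shows while the player is within HealthRadius, with Tick updating its fill and turning it toward the camera.
; On defeat it awards Exp to the player, updates the wave game mode's DHV count, plays a random death sound and destroys itself after a delay.
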(event `OnDefeated`
  (set `self.IsDefeated` true)
  (`/Game/Blueprint/Character/caption/BP_Caption.AddExp` (`self.die`) (`self.Exp`))
  (`self.Update DHV`)
  (`self.PlayDeathSound`)
  (`PrimitiveComponent.SetCollisionEnabled` (`self.CapsuleComponent`) "NoCollision")
  (`KismetSystemLibrary.Delay` 2.0)
  (`self.K2_DestroyActor`)
  (`self.OnElminated`))

(event `self.ReceiveBeginPlay`
  (`parent.ReceiveBeginPlay`)
  (`|ExecutionSequence`
    (:`then_0`
      (add `self.Defeated` (delegate `OnDefeated`)))
    (:`then_1`
      (bind _asbp_caption (cast `/Game/Blueprint/Character/caption/BP_Caption` (`GameplayStatics.GetPlayerCharacter` 0)))
      (set `self.die` _asbp_caption))))

(event `self.AggroRange.OnComponentBeginOverlap`
  (params (OverlappedComponent :type "PrimitiveComponent Object Reference") (OtherActor :type "Actor Object Reference") (OtherComp :type "PrimitiveComponent Object Reference") (OtherBodyIndex :type Integer) (bFromSweep :type Boolean) (SweepResult :type "HitResult Structure (by ref)"))
  (bind _asbp_caption (cast `/Game/Blueprint/Character/caption/BP_Caption` OtherActor))
  (bind _asaic_enemy (cast `/Game/Blueprint/AI/AIC_Enemy` (`AIBlueprintHelperLibrary.GetAIController` self)))
  (`/Game/Blueprint/AI/AIC_Enemy.SetAttackTarget` _asaic_enemy _asbp_caption))

(event `self.ReceiveTick`
  (params (DeltaSeconds :type "Float (single-precision)"))
  (bind _healthbarwidget (`self.HealthBarWidget`))
  (bind _aswb_npc_health (cast `/Game/Widget/WB_NPC_Health` (`WidgetComponent.GetUserWidgetObject` (`self.HealthBarWidget`))))
  (`ProgressBar.SetPercent` (`/Game/Widget/WB_NPC_Health.HealthBar` _aswb_npc_health) (/ (`self.CurrentHealth`) (`self.MaxHealth`)))
  (`SceneComponent.K2_SetWorldRotation` _healthbarwidget (`KismetMathLibrary.FindLookAtRotation` (`SceneComponent.K2_GetComponentLocation` _healthbarwidget) (`SceneComponent.K2_GetComponentLocation` (`PlayerCameraManager.TransformComponent` (`GameplayStatics.GetPlayerCameraManager` 0)))) false false))

(event `self.HealthRadius.OnComponentBeginOverlap`
  (params (OverlappedComponent :type "PrimitiveComponent Object Reference") (OtherActor :type "Actor Object Reference") (OtherComp :type "PrimitiveComponent Object Reference") (OtherBodyIndex :type Integer) (bFromSweep :type Boolean) (SweepResult :type "HitResult Structure (by ref)"))
  (cast `/Game/Blueprint/Character/caption/BP_Caption` OtherActor)
  (`SceneComponent.SetVisibility` (`self.HealthBarWidget`) true false))

(event `self.HealthRadius.OnComponentEndOverlap`
  (params (OverlappedComponent :type "PrimitiveComponent Object Reference") (OtherActor :type "Actor Object Reference") (OtherComp :type "PrimitiveComponent Object Reference") (OtherBodyIndex :type Integer))
  (cast `/Game/Blueprint/Character/caption/BP_Caption` OtherActor)
  (`SceneComponent.SetVisibility` (`self.HealthBarWidget`) false false))

(fn `PlayDeathSound`
  (bind _deathsfx (`self.DeathSFX`))
  (`GameplayStatics.PlaySoundAtLocation` (`|GetArrayItem` _deathsfx (`.OutIndex` (`KismetArrayLibrary.Array_Random` _deathsfx))) (`self.K2_GetActorLocation`) (struct) 1.0 1.0 0.0 null null null null))

(fn `Update DHV`
  (bind _wave_game_mode (`/Game/Blueprint/BP_FuntionLibrary.GetWaveGameMode`))
  (bind _dhv (`self.DHV`))
  (set `/Game/Blueprint/GM_Action.DHVCollected` (`KismetMathLibrary.And_IntInt` (+ _dhv (`self.DHVCollectedShar`)) (+ _dhv (`/Game/Blueprint/GM_Action.DHVCollected` _wave_game_mode))) _wave_game_mode))

(fn `UserConstructionScript`
  (`parent.UserConstructionScript`))