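; GM_Action is the game mode for shark-killing waves, creating HUD and quest widgets and showing WB_GameLose once the wave number reaches six.
; Each wave loads a shark pool from DT_SharkData and queues random types at random spawners up to SharkLimit, replenishing on kills.
; Clearing the pool or running out the countdown triggers a timed interlude that clears spawners before the next wave.
; The formula-based AlgorithmicWave builder is never run.
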(event `self.ReceiveBeginPlay`
  (`|ExecutionSequence`
    (:`then_0`
      (bind _returnvalue (`|CreateWidget` "/Game/Widget/WBP_HUD.WBP_HUD_C"))
      (bind _output_get (set `self.HUDWidget` _returnvalue))
      (`UserWidget.AddToViewport` _output_get 0))
    (:`then_3`
      (bind _returnvalue_2 (`|CreateWidget` "/Game/Widget/WB_WaveHUB.WB_WaveHUB_C"))
      (set `self.WaveStart` _returnvalue_2))
    (:`then_6`
      (bind _returnvalue_3 (`|CreateWidget` "/Game/Widget/WB_Quest.WB_Quest_C"))
      (bind _output_get_2 (set `self.Objectives Widget REF` _returnvalue_3))
      (`UserWidget.AddToViewport` _output_get_2 0)
      (`Widget.SetVisibility` (`/Game/Widget/WB_Quest.TextBlock_102` _output_get_2) "Hidden"))))

(event `Slide On`
  (`/Game/Widget/WB_Quest.Slide On` (`self.Objectives Widget REF`)))

(event `Interlude`
  (bind _returnvalue (`KismetSystemLibrary.K2_SetTimerDelegate` (delegate `BeginNextWave`) 10.0))
  (set `self.InterludeTimer` _returnvalue)
  (`self.EndWave`))

(event `Slide Off`
  (`/Game/Widget/WB_Quest.Slide Off` (`self.Objectives Widget REF`)))

(event `Resetimer`
  (goto _label :!via `Reset`))

(event `BeginNextWave`
  (`self.StarWave`))

(event `QuestMisstion`
  (`/Game/Widget/WB_Quest.QuestMisstion` (`self.Objectives Widget REF`)))

(event `StartTimer`
  (if (== (`self.Seconds`) 0)
    (if (== (`self.Minutes`) 0)
      (`/Engine/EditorBlueprintResources/StandardMacros.DoOnce` false :!label _label
        (:`Completed`
          (if (not (`self.OnBreak`))
            (`self.Interlude`)
            (else
              (set `self.OnBreak` false)))))
      (else
        (set `self.Seconds` 59)
        (set `self.Minutes` (- (`self.Minutes`) 1))
        (`self.OnTimerUpdated` (`self.Minutes`) (`self.Seconds`) :!label _label_2)))
    (else
      (set `self.Seconds` (- (`self.Seconds`) 1))
      (goto _label_2))))

(fn `AddSharkToQueue`
  (`/Game/Blueprint/Event/SpawnShark/BP_SpawnShark.AddSharkToQueue` (`KismetArrayLibrary.Array_Random` (`self.SharkSpawners`)) (`self.GetSharkFromPool`)))

(fn `AlgorithmicWave`
  (bind _sharkpoolsize (`self.GetPoolSize`))
  (bind _wavenumber (`self.WaveNumber`))
  (`BlueprintMapLibrary.Map_Add` (`self.SharkPool`) "/Game/Blueprint/Character/Shark/BP_SharkRed.BP_SharkRed_C" (`KismetMathLibrary.Clamp` (+ (* _wavenumber _wavenumber) 2) 10))
  (`BlueprintMapLibrary.Map_Add` (`self.SharkPool`) "/Game/Blueprint/Character/Shark/BP_SharkBlue.BP_SharkBlue_C" (`KismetMathLibrary.Clamp` (+ (* (`self.WaveNumber`) 1) 2) 8))
  (`BlueprintMapLibrary.Map_Add` (`self.SharkPool`) "/Game/Blueprint/Character/Shark/BP_SharkBlack.BP_SharkBlack_C" (* (`self.WaveNumber`) 1))
  (set `self.SharkRemaining` _sharkpoolsize)
  (set `self.TotalShark` _sharkpoolsize))

(fn `BuildSharkPool`
  (bind _sharkpoolsize (`self.GetPoolSize`))
  (bind _returnvalue (`|GetDataTableRow` "/Game/DataTable/WaveData/DT_SharkData.DT_SharkData" (`KismetStringLibrary.Conv_StringToName` (`KismetStringLibrary.Conv_IntToString` (`self.WaveNumber`))))
    (:`then`
      (set `self.SharkPool` (`.SharkPool_4_06FCADB24002E7A3ED6EF2934D2DBF74` (break `/Game/DataTable/WaveData/S_waveInfo` _returnvalue)))
      (set `self.SharkRemaining` _sharkpoolsize)
      (set `self.TotalShark` _sharkpoolsize))))

(fn `BuildWave`
  (`self.BuildSharkPool`)
  (for _ (range (+ (- (`KismetMathLibrary.Min` (`self.GetPoolSize`) (`self.SharkLimit`)) 0) 1))
    (`self.AddSharkToQueue`)))

(fn `CountDownTimer`
  (returns (Minutes :type Integer) (Seconds :type Integer))
  (`KismetSystemLibrary.K2_SetTimerDelegate` (`|CreateDelegate` :!event `StartTimer`) 1.0 true)
  (return (`self.Minutes`) (`self.Seconds`)))

(fn `CreateWaveHUB`
  (bind _returnvalue (`|CreateWidget` "/Game/Widget/WB_WaveHUB.WB_WaveHUB_C"))
  (`UserWidget.AddToViewport` _returnvalue 0))

(fn `EndWave`
  (set `self.SharkKilled` 0)
  (set `self.Minutes` 0)
  (set `self.Seconds` 0)
  (for _array_element (`self.SharkSpawners`)
    (`/Game/Blueprint/Event/SpawnShark/BP_SpawnShark.Clear All Shark` _array_element))
  (`self.OnWaveEnd`))

(fn `GetPoolSize`
  (returns (SharkPoolSize :type Integer))
  (locals (Local_SharkPool :type Integer))
  (bind _values (`BlueprintMapLibrary.Map_Values` (`self.SharkPool`)))
  (for _array_element _values
    (set `local.Local_SharkPool` (+ _array_element (`local.Local_SharkPool`))))
  (return (`local.Local_SharkPool`)))

(fn `GetSharkFromPool`
  (returns (SharkClass :type "/Game/Blueprint/Character/Shark/BP_Shark Class Reference"))
  (locals (Local_SharkClass :type "/Game/Blueprint/Character/Shark/BP_Shark Class Reference"))
  (bind _keys (`BlueprintMapLibrary.Map_Keys` (`self.SharkPool`)))
  (bind _output_get (set `local.Local_SharkClass` (`KismetArrayLibrary.Array_Random` _keys)))
  (bind _returnvalue (- (`BlueprintMapLibrary.Map_Find` (`self.SharkPool`) _output_get) 1))
  (if (<= _returnvalue 0)
    (`BlueprintMapLibrary.Map_Remove` (`self.SharkPool`) (`local.Local_SharkClass`))
    (else
      (`BlueprintMapLibrary.Map_Add` (`self.SharkPool`) (`local.Local_SharkClass`) _returnvalue)))
  (return (`local.Local_SharkClass`)))

(fn `GetSharkLimid`
  (set `self.SharkLimit` (`KismetMathLibrary.Clamp` (+ (`self.SharkLimit`) 1) 5 (/ (`self.WaveNumber`) 1))))

(fn `GetSharkSpawners`
  (bind _outactors (`GameplayStatics.GetAllActorsOfClass` "/Game/Blueprint/Event/SpawnShark/BP_SpawnShark.BP_SpawnShark_C"))
  (set `self.SharkSpawners` _outactors))

(fn `OnSharkEliminated`
  (`/Engine/EditorBlueprintResources/StandardMacros.DecrementInt` (`self.SharkRemaining`)
    (:`  `
      (bind _result (`/Engine/EditorBlueprintResources/StandardMacros.IncrementInt` (`self.SharkKilled`))
        (:`  `
          (`self.OnSharkKilled` _result (`self.TotalShark`) (`self.DHVCollected`))
          (if (< (`self.SharkRemaining`) (`self.SharkLimit`))
            (if (== (`self.SharkRemaining`) 0)
              (bind _result_2 (`/Engine/EditorBlueprintResources/StandardMacros.IncrementInt` (+ (`self.DHVCollected`) 25))
                (:`  `
                  (set `self.DHVCollected` _result_2)
                  (`self.Interlude`)
                  (set `self.OnBreak` true))))
            (else
              (`self.AddSharkToQueue`))))))))

(fn `RestartGame`
  (bind _returnvalue (`GameplayStatics.GetCurrentLevelName` true))
  (`GameplayStatics.OpenLevel` (`KismetStringLibrary.Conv_StringToName` _returnvalue)))

(fn `StarWave`
  (bind _returnvalue (`GameplayStatics.GetPlayerController` 0))
  (`/Engine/EditorBlueprintResources/StandardMacros.IncrementInt` (`self.WaveNumber`)
    (:`  `
      (if (>= (`self.WaveNumber`) 6)
        (bind _returnvalue_2 (`|CreateWidget` "/Game/Widget/WB_GameLose.WB_GameLose_C"))
        (`UserWidget.AddToViewport` _returnvalue_2 0)
        (set `PlayerController.bShowMouseCursor` true _returnvalue)
        (`WidgetBlueprintLibrary.SetInputMode_GameAndUIEx` _returnvalue _returnvalue_2)
        (else
          (`self.GetSharkLimid`)
          (`self.GetSharkSpawners`)
          (`self.WaveClock`)
          (`self.BuildWave`)
          (`self.OnStartWave` (`self.WaveNumber`) (`self.SharkKilled`) (`self.TotalShark`) (`self.DHVCollected`))
          (`self.Resetimer`))))))

(fn `UserConstructionScript`)

(fn `WaveClock`
  (bind _output_get (set `self.StoredSeconds` (+ (`self.StoredSeconds`) 120)))
  (if (>= _output_get 60)
    (set `self.StoredSeconds` 0)
    (bind _result (`/Engine/EditorBlueprintResources/StandardMacros.IncrementInt` (`self.StoredMinutes`))
      (:`  `
        (set `self.Minutes` _result)))
    (else
      (set `self.Seconds` (`self.StoredSeconds`))
      (set `self.Minutes` (`self.StoredMinutes`)))))