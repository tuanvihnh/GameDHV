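; BP_GoalnoCube is a one-shot trigger box that starts a wave interlude when a BP_Caption actor overlaps it.
; After a short delay, it casts the game mode to GM_Action and stores it as WaveStar.
; It hides that game mode's root component, calls CreateWaveHUB and Interlude on it, then plays the Hanhdon sound in 2D.
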(event `self.Box.OnComponentBeginOverlap`
  (params (OverlappedComponent :type "PrimitiveComponent Object Reference") (OtherActor :type "Actor Object Reference") (OtherComp :type "PrimitiveComponent Object Reference") (OtherBodyIndex :type Integer) (bFromSweep :type Boolean) (SweepResult :type "HitResult Structure (by ref)"))
  (bind _wavestar (`self.WaveStar`))
  (cast `/Game/Blueprint/Character/caption/BP_Caption` OtherActor)
  (`/Engine/EditorBlueprintResources/StandardMacros.DoOnce` false
    (:`Completed`
      (`KismetSystemLibrary.Delay` 2.0)
      (bind _asgm_action (cast `/Game/Blueprint/GM_Action` (`GameplayStatics.GetGameMode`)))
      (bind _output_get (set `self.WaveStar` _asgm_action))
      (`SceneComponent.SetVisibility` (`/Game/Blueprint/GM_Action.DefaultSceneRoot` _output_get) false false)
      (`/Game/Blueprint/GM_Action.CreateWaveHUB` _wavestar)
      (`/Game/Blueprint/GM_Action.Interlude` _wavestar)
      (`GameplayStatics.PlaySound2D` "/Game/Sounds/Hanhdon.Hanhdon" 1.0 1.0 0.0 null null))))

(fn `UserConstructionScript`)